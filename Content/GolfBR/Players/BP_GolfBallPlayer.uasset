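; Golf-ball player character for GolfBR, a work-in-progress mix of physics impulses and networked character launches.
; Q pushes the ball upward, and Dash both pushes it along the camera's forward vector and fires a cooldown-gated server/multicast LaunchCharacter with placeholder velocity.
; LaunchBall is meant to turn timeline charge and movement axes into a camera-yaw-relative impulse.
; Charge, jump, setup and UI wiring are disconnected, as is CalculateChargeDirection's math.
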(event Custom|Launch%20Ball
  (bind _right_axis (Variables|Default|GetRight%20Axis))
  (bind _charge (Variables|Default|GetCharge))
  (bind _forward_axis (Variables|Default|GetForward%20Axis))
  (bind _charge_2 (Variables|Default|GetCharge))
  (bind _charge_3 (Variables|Default|GetCharge))
  (bind (_x _y) (Utilities|CalculateChargeDirection _right_axis _charge_2 1e+03 0.0))
  (bind (_x_2 _y_2) (Utilities|CalculateChargeDirection _forward_axis _charge_3 1e+03 0.0))
  (bind _returnvalue (+ _y_2 _y))
  (bind _returnvalue_2 (+ _x_2 _x))
  (if (and (> _charge 0.0) (> (+ (Math|Float|Absolute(Float) (Variables|Default|GetForward%20Axis)) (Math|Float|Absolute(Float) (Variables|Default|GetRight%20Axis))) 0.0))
    (Development|PrintString (Utilities|String|Append "charge:  " (Utilities|String|ToString(Float) _charge) "| x: " (Utilities|String|ToString(Float) _forward_axis) "| y:" (Utilities|String|ToString(Float) _right_axis)))
    (Development|PrintString (Utilities|String|Append "x:  " (Utilities|String|ToString(Float) _returnvalue_2) "| y: " (Utilities|String|ToString(Float) _returnvalue)))
    (Physics|AddImpulse (Variables|Default|GetGolfBall) (Math|Vector|MakeVector (* 1 _returnvalue_2) (* 1 _returnvalue) 0.0) "None" false)))

(event Custom|Set%20Cooldown)

(event Custom|Dash%20Multicast
  (params (Target :type Primitive%20Component%20Object%20Reference) (New%20Vel%20X :type Float%20%28single-precision%29) (New%20Vel%20Y :type Float%20%28single-precision%29))
  (Character|LaunchCharacter (Math|Vector|MakeVector New%20Vel%20X New%20Vel%20Y 0.0) false false))

(event Custom|Dash%20Server
  (params (Target :type Primitive%20Component%20Object%20Reference) (New%20Vel%20X :type Float%20%28single-precision%29) (New%20Vel%20Y :type Float%20%28single-precision%29))
  (Character|LaunchCharacter (Math|Vector|MakeVector New%20Vel%20X New%20Vel%20X 0.0) false false))

(event Custom|Jump%20Multicast
  (params (Target :type Primitive%20Component%20Object%20Reference))
  (Physics|AddImpulse Target (Math|Vector|MakeVector 0.0 0.0 5e+02) "None" true)
  (Development|PrintString "Hello"))

(event Custom|Jump%20Server
  (params (Target :type Primitive%20Component%20Object%20Reference))
  (Development|PrintString "Hello"))

(event Custom|CheckCharge)

(event Custom|End%20Cooldown
  (bind _newtrack_0 (Timeline|Timeline_1 SetNewTime)
    (:Update
      (Variables|Default|SetCooldown _newtrack_0))))

(event Custom|Dash%20Cooldown
  (CallFunction|StopCharge)
  (bind _newtrack_0 (Timeline|Timeline_1 PlayFromStart)
    (:Update
      (Variables|Default|SetCooldown _newtrack_0))))

(event Custom|Stop%20Charge
  (Utilities|FlowControl|Sequence
    (:then_0
      (bind _newtrack_0 (Timeline|Timeline_0 Stop)
        (:Update
          (Variables|Default|SetCharge _newtrack_0))))
    (:then_1
      (Timeline|Timeline_0 SetNewTime))))

(event Custom|Launch%20Multicast
  (params (New%20Vel%20X :type Float%20%28single-precision%29) (New%20Vel%20Y :type Float%20%28single-precision%29) (Target :type Primitive%20Component%20Object%20Reference))
  (Character|LaunchCharacter (Math|Vector|MakeVector New%20Vel%20X New%20Vel%20Y 0.0) false false))

(event Custom|Launch%20Server
  (params (New%20Vel%20X :type Float%20%28single-precision%29) (New%20Vel%20Y :type Float%20%28single-precision%29) (Target :type Primitive%20Component%20Object%20Reference))
  (Character|LaunchCharacter (Math|Vector|MakeVector New%20Vel%20X New%20Vel%20Y 0.0) false false))

(event EventBeginPlay)

(event Input|ActionEvents|InputActionCharge
  (params (Key :type Key%20Structure :default "None")))

(event Input|ActionEvents|InputActionDash
  (params (Key :type Key%20Structure :default "None"))
  (bind _returnvalue (+ 0.0 1.0))
  (bind _returnvalue_2 (+ 0.0 1.0))
  (bind _ball (Variables|Default|GetBall))
  (:Pressed
    (if (not (> (Variables|Default|GetCooldown) 0.0))
      (if (> (+ (Math|Float|Absolute(Float) (Variables|Default|GetForward%20Axis)) (Math|Float|Absolute(Float) (Variables|Default|GetRight%20Axis))) 0.0)
        (CallFunction|DashCooldown)
        (Networking|SwitchHasAuthority
          (:Authority
            (CallFunction|DashMulticast _ball _returnvalue _returnvalue_2))
          (:Remote
            (CallFunction|DashServer _ball _returnvalue _returnvalue_2)))))))

(event Input|ActionEvents|InputActionDash
  (params (Key :type Key%20Structure :default "None"))
  (:Pressed
    (Physics|AddImpulse (Variables|Default|GetGolfBall) (* (Math|Vector|GetForwardVector (Variables|Default|GetFollowCamera)) 1000) "None" false)))

(event Input|AxisEvents|InputAxisMoveForward
  (params (AxisValue :type Float%20%28single-precision%29))
  (Variables|Default|SetForward%20Axis AxisValue))

(event Input|AxisEvents|InputAxisMoveRight
  (params (AxisValue :type Float%20%28single-precision%29))
  (Variables|Default|SetRight%20Axis AxisValue))

(event Input|KeyboardEvents|Q
  (params (Key :type Key%20Structure :default "None"))
  (:Pressed
    (Physics|AddImpulse (Variables|Default|GetGolfBall) "0, 0,1000.000000" "None" false)))

(fn ConstructionScript)