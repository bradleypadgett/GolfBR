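; BP_testphysx is a physics test Blueprint that launches a static mesh and shows elapsed time on screen.
; BeginPlay and the F key zero the timer, apply a horizontal velocity-change impulse along camera forward, and play a timeline.
; The timeline's event track counts time in fixed increments, Tick prints it, and stoptimer halts it.
; R returns the mesh to a fixed location and clears its velocities.
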(event Custom|stop%20timer
  (Timeline|Timeline_0 Stop
    (:NewTrack_1
      (Variables|Default|Settime%20elapsed (+ (Variables|Default|Gettime%20elapsed) 0.01)))))

(event EventTick
  (params (DeltaSeconds :type Float%20%28single-precision%29))
  (Development|PrintString (Utilities|String|Append "Time elapsed: " (Utilities|String|ToString(Float) (Variables|Default|Gettime%20elapsed)) " seconds") true true "(R=0.000000,G=0.660000,B=1.000000,A=1.000000)" DeltaSeconds))

(event EventBeginPlay
  (bind _camera (Variables|Default|GetCamera))
  (bind _returnvalue (Math|Vector|GetForwardVector _camera))
  (Variables|Default|Settime%20elapsed 0.0)
  (Utilities|FlowControl|Sequence
    (:then_0
      (Physics|AddImpulse (Variables|Default|GetStaticMesh) (* (Math|Vector|MakeVector (.x _returnvalue) (.y _returnvalue) 0.0) 1000) "None" true))
    (:then_1
      (Timeline|Timeline_0 Play
        (:NewTrack_1
          (Variables|Default|Settime%20elapsed (+ (Variables|Default|Gettime%20elapsed) 0.01)))))))

(event Input|KeyboardEvents|R
  (params (Key :type Key%20Structure :default "None"))
  (bind _staticmesh (Variables|Default|GetStaticMesh))
  (:Pressed
    (Transformation|SetWorldLocation _staticmesh "0, 0,20.000000" false false)
    (Physics|SetPhysicsLinearVelocity _staticmesh "0, 0, 0" false "None")
    (Class|PrimitiveComponent|SetPhysicsAngularVelocityinDegrees _staticmesh "0, 0, 0" false "None")))

(event Input|KeyboardEvents|F
  (params (Key :type Key%20Structure :default "None"))
  (bind _camera (Variables|Default|GetCamera))
  (bind _returnvalue (Math|Vector|GetForwardVector _camera))
  (:Pressed
    (Variables|Default|Settime%20elapsed 0.0)
    (Utilities|FlowControl|Sequence
      (:then_0
        (Physics|AddImpulse (Variables|Default|GetStaticMesh) (* (Math|Vector|MakeVector (.x _returnvalue) (.y _returnvalue) 0.0) 1000) "None" true))
      (:then_1
        (Timeline|Timeline_0 Play
          (:NewTrack_1
            (Variables|Default|Settime%20elapsed (+ (Variables|Default|Gettime%20elapsed) 0.01))))))))

(fn ConstructionScript)