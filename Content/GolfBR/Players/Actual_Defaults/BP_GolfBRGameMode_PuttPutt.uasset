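; Game mode Blueprint, named for the PuttPutt mode of GolfBR, that currently adds only debug output on BeginPlay.
; After calling the parent BeginPlay, it prints the GameState PlayerArray length, then that count minus a rounded quarter of it.
; The computed value is only printed, never stored or applied, and the construction script just calls its parent.
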(event EventBeginPlay
  (bind _returnvalue (Game|GetGameState))
  (bind _playerarray (Variables|/Script/Engine.GameStateBase|GetPlayerArray _returnvalue))
  (bind _returnvalue_2 (Utilities|Array|Length _playerarray))
  (|CallParentFunction)
  (Development|PrintString (Utilities|String|ToString(Integer) _returnvalue_2) true true "(R=1.000000,G=0.000000,B=0.442750,A=1.000000)")
  (Development|PrintString (Utilities|String|ToString(Integer) (- _returnvalue_2 (Math|Float|Round (/ (Math|Conversions|ToFloat(Integer) _returnvalue_2) 4.0))))))

(fn ConstructionScript
  (|CallParentFunction))