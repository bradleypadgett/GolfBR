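; Game mode for the GolfBR game that handles player joins and spawn point selection.
; On PostLogin it gives the new player state a default name built from "Player" and the current player count.
; ChoosePlayerStart returns the first PlayerStart not tagged "Taken" and tags it so no two players share a start.
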(event EventPostLogin
  (params (NewPlayer :type Player%20Controller%20Object%20Reference))
  (bind _asbp_golf_brplayer_state (Utilities|Casting|CastToBP_GolfBRPlayerState (Variables|/Script/Engine.Controller|GetPlayerState NewPlayer)))
  (Class|GolfBRPlayerState|SetPlayerNameExposed _asbp_golf_brplayer_state (Utilities|String|Append "Player " (Utilities|String|ToString(Integer) (Utilities|Array|Length (Variables|/Script/Engine.GameStateBase|GetPlayerArray (Game|GetGameState)))))))

(fn ConstructionScript)

(fn ChoosePlayerStart
  (params (Player :type Controller%20Object%20Reference))
  (bind _outactors (Actor|GetAllActorsOfClass "/Script/Engine.PlayerStart"))
  (bind _array_element (Utilities|Array|ForEachLoopwithBreak _outactors :!label _label)
    (:LoopBody
      (if (Utilities|Name|NotEqual(Name) (Variables|/Script/Engine.PlayerStart|GetPlayerStartTag _array_element) "Taken")
        (Variables|/Script/Engine.PlayerStart|SetPlayerStartTag _array_element "Taken")
        (Utilities|FlowControl|Sequence
          (:then_0
            (return _array_element))
          (:then_1
            (goto _label Break)))))))