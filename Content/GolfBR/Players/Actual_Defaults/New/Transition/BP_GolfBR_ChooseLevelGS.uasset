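; Game state for the GolfBR between-round level selection screen, which picks the next map or declares a winner.
; It has each player state add the choosing UI, then counts players who are not permanent spectators.
; With several left, a timeline animates the status text, maps the count to a hardcoded level, shows its mode name and issues a ServerTravel command.
; With one or none, it shows the first named player as winner and opens the main menu.
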(event Custom|Set%20Choosing%20Level%20UI%20Timer
  (Variables|Default|SetReal%20Player%20Amount 0)
  (for _array_element (Variables|Default|GetPlayerArray)
    (bind _asbp_golf_brplayer_state (Utilities|Casting|CastToBP_GolfBRPlayerState _array_element))
    (Development|PrintString "dvjnnjpvjnkadnjkdav")
    (if (not (Variables|/Game/GolfBR/Players/Actual_Defaults/New/BP_GolfBRPlayerState.BP_GolfBRPlayerState_C|GetPermanantSpectator _asbp_golf_brplayer_state))
      (Math|Integer|IncrementInt (Variables|Default|GetReal%20Player%20Amount))))
  (if (<= (Variables|Default|GetReal%20Player%20Amount) 1)
    (CallFunction|ChooseWinner)
    (else
      (Variables|Default|SetLevel%20Text 0)
      (Timeline|Choosing%20Level%20Text%20Timer PlayFromStart
        (:Finished
          (bind _asgm_choose_level (Utilities|Casting|CastToGM_ChooseLevel (Game|GetGameMode)))
          (bind _output_get (Variables|Default|SetLevel%20Chosen (Utilities|Select :Index (Variables|Default|GetReal%20Player%20Amount) :Option%200 "" :Option%201 (Variables|Default|GetLevel%20Chosen) :Option%202 "L_FallingPlatforms_1" :Option%203 "L_SwingArm_1" :Option%204 "L_PuttPutt_3" :Option%205 "L_PuttPutt_1" :Option%206 "L_PuttPutt_2" :Option%207 "L_PuttPutt_3" :Option%208 "L_PuttPutt_2")))
          (Utilities|FlowControl|Sequence
            (:then_0
              (switch string _output_get
                (:Default
                  (Variables|Default|SetChoose%20Level%20Text "idk"))
                (:L_PuttPutt_1
                  (Variables|Default|SetChoose%20Level%20Text "Putt-Race!" :!label _label))
                (:L_PuttPutt_2
                  (goto _label))
                (:L_SwingArm_1
                  (Variables|Default|SetChoose%20Level%20Text "Sweeper Run!"))
                (:L_FallingPlatforms_1
                  (Variables|Default|SetChoose%20Level%20Text "Floor Fall!"))
                (:L_PuttPutt_3
                  (goto _label))))
            (:then_1
              (Utilities|FlowControl|Delay 2.0)
              (Development|ExecuteConsoleCommand (Utilities|String|Append "ServerTravel" " " (Variables|Default|GetLevel%20Chosen)) 0))))
        (:NewTrack_0
          (Math|Integer|IncrementInt (Variables|Default|GetLevel%20Text)
            (:%20%20
              (Variables|Default|SetChoose%20Level%20Text (Utilities|Select :Index (Variables|Default|GetLevel%20Text) :Option%200 "?" :Option%201 "Choosing Level ." :Option%202 "Choosing Level .." :Option%203 "Choosing Level ..." :Option%204 ".")))))))))

(event Custom|Choose%20Winner
  (bind _array_element (Utilities|Array|ForEachLoopwithBreak (Variables|Default|GetPlayerArray) :!label _label)
    (:LoopBody
      (if (not (Utilities|Array|IsEmpty (PlayerState|GetPlayerName _array_element)))
        (Variables|Default|SetChoose%20Level%20Text (Utilities|String|Append (PlayerState|GetPlayerName _array_element) " wins!"))
        (goto _label Break)))
    (:Completed
      (Utilities|FlowControl|Delay 5.0)
      (CallFunction|GoBack))))

(event Custom|Go%20back
  (Game|OpenLevel(byName) "MainMenuMap"))

(event Custom|Add%20Choosing%20Level%20UI
  (for _array_element (Variables|Default|GetPlayerArray)
    (bind _asbp_golf_brplayer_state (Utilities|Casting|CastToBP_GolfBRPlayerState _array_element))
    (Default|AddChooseLevelUIfromGM _asbp_golf_brplayer_state)))

(event EventBeginPlay)

(event EventTick
  (params (DeltaSeconds :type Float%20%28single-precision%29)))

(fn ConstructionScript)