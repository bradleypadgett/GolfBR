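; Base game mode for GolfBR, an elimination golf game played in rounds.
; The match starts once no players are still travelling, resetting each player's qualified flag, and spawning claims PlayerStarts by tagging them "Taken".
; On round end, the game state sets unqualified players, then the mode server-travels to the level-choice map, or quits when one or fewer non-permanent-spectators remain or only one player is connected.
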(event Custom|Round%20Ended
  (bind _returnvalue (Game|GetGameState))
  (bind _playerarray (Variables|/Script/Engine.GameStateBase|GetPlayerArray _returnvalue))
  (Development|PrintString "Round Ended!")
  (bind _asbp_golf_br_gs (Utilities|Casting|CastToBP_GolfBR_GS (Game|GetGameState)))
  (Default|SetUnqualifiedPlayers _asbp_golf_br_gs)
  (Variables|Default|Setcheck%20amount%20of%20players%20left 0)
  (if (== (Utilities|Array|Length _playerarray) 1)
    (Game|QuitGame 0 "Quit" false :!label _label)
    (else
      (for _array_element _playerarray
        (bind _asbp_golf_brplayer_state (Utilities|Casting|CastToBP_GolfBRPlayerState _array_element))
        (if (not (Variables|/Game/GolfBR/Players/Actual_Defaults/New/BP_GolfBRPlayerState.BP_GolfBRPlayerState_C|GetPermanantSpectator _asbp_golf_brplayer_state))
          (Math|Integer|IncrementInt (Variables|Default|Getcheck%20amount%20of%20players%20left))))
      (if (<= (Variables|Default|Getcheck%20amount%20of%20players%20left) 1)
        (goto _label)
        (else
          (Development|ExecuteConsoleCommand "ServerTravel L_ChooseLevelMap" 0))))))

(event Custom|Check%20Winner)

(event Custom|Get%20New%20Level)

(event EventBeginPlay)

(event EventPostLogin
  (params (NewPlayer :type Player%20Controller%20Object%20Reference)))

(event EventOnLogout
  (params (ExitingController :type Controller%20Object%20Reference))
  (|CallParentFunction ExitingController))

(event EventBPHandleMatchHasStarted
  (for _array_element (Variables|/Script/Engine.GameStateBase|GetPlayerArray (Game|GetGameState))
    (bind _asbp_golf_brplayer_state (Utilities|Casting|CastToBP_GolfBRPlayerState _array_element))
    (Variables|/Game/GolfBR/Players/Actual_Defaults/New/BP_GolfBRPlayerState.BP_GolfBRPlayerState_C|SetQualifiedRound _asbp_golf_brplayer_state false)))

(fn ConstructionScript)

(fn ChoosePlayerStart
  (params (Player :type Controller%20Object%20Reference))
  (bind _outactors (Actor|GetAllActorsOfClass "/Script/Engine.PlayerStart"))
  (bind _array_element (Utilities|Array|ForEachLoopwithBreak _outactors :!label _label)
    (:LoopBody
      (if (Utilities|Name|NotEqual(Name) (Variables|/Script/Engine.PlayerStart|GetPlayerStartTag _array_element) "Taken")
        (Variables|/Script/Engine.PlayerStart|SetPlayerStartTag _array_element "Taken")
        (Utilities|FlowControl|Sequence
          (:then_0
            (return _array_element))
          (:then_1
            (goto _label Break)))))))

(fn ReadytoStartMatch
  (return (== (Variables|Default|GetNumTravellingPlayers) 0)))