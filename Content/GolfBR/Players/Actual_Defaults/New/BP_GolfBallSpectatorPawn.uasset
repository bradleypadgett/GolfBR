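; Spectator pawn for the golf battle royale that follows active players by snap-attaching itself to their pawns, with mouse look through controller yaw and pitch.
; On BeginPlay it attaches to the first non-spectator in the PlayerArray (despite the "Random" name), and a looping timer re-picks when that target becomes invalid or spectates.
; Left and right mouse cycle forward and backward through non-spectating players, wrapping around.
; Spectator UI and server-set logic are empty or unwired.
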(event Custom|Server%20Set
  (params (Player :type Integer) (bUp :type Boolean)))

(event Custom|Initialize%20Spectator
  (bind _returnvalue (Pawn|GetController))
  (bind _playerstate (Variables|/Script/Engine.Controller|GetPlayerState _returnvalue))
  (bind _pawnprivate (Variables|/Script/Engine.PlayerState|GetPawnPrivate _playerstate))
  (bind _outactors (Actor|GetAttachedActors _pawnprivate true))
  (Development|PrintString (Utilities|String|ToString(Integer) (Utilities|Array|Length _outactors)))
  (for _array_element _outactors
    (Development|PrintString (Utilities|GetDisplayName _array_element) true true "(R=0.546875,G=0.122477,B=0.200780,A=1.000000)")
    (if (== (Utilities|GetClass _array_element) "BP_GolfBallSpectatorPawn_C")
      (bind _asbp_golf_ball_spectator_pawn (Utilities|Casting|CastToBP_GolfBallSpectatorPawn _array_element))
      (CallFunction|SetRandomSpectator _asbp_golf_ball_spectator_pawn))))

(event Custom|Set%20Permanant%20Spectating%20UI)

(event Custom|Set%20Random%20Spectator
  (bind _returnvalue (Game|GetGameState))
  (Utilities|IsValid _returnvalue
    (:Is%20Valid
      (bind _array_element (Utilities|Array|ForEachLoopwithBreak (Variables|/Script/Engine.GameStateBase|GetPlayerArray _returnvalue) :!label _label)
        (:LoopBody
          (if (not (Variables|/Script/Engine.PlayerState|GetbIsSpectator _array_element))
            (Utilities|FlowControl|Sequence
              (:then_0
                (goto _label Break))
              (:then_1
                (Transformation|AttachActorToActor (Variables|/Script/Engine.PlayerState|GetPawnPrivate _array_element) "None" "SnapToTarget" "SnapToTarget" "SnapToTarget" true)))))))))

(event Custom|Check%20If%20Spectator%20is%20Valid
  (bind _returnvalue (Actor|GetAttachParentActor))
  (Utilities|IsValid _returnvalue
    (:Is%20Valid
      (bind _asbp_my_golf_ball_player (Utilities|Casting|CastToBP_MyGolfBallPlayer _returnvalue)
        (:then
          (bind _playerstate (Variables|/Script/Engine.Pawn|GetPlayerState _asbp_my_golf_ball_player)
            (:then
              (if (Variables|/Script/Engine.PlayerState|GetbIsSpectator _playerstate)
                (CallFunction|SetRandomSpectator :!label _label)))
            (:else
              (goto _label))))
        (:CastFailed
          (goto _label))))
    (:Is%20Not%20Valid
      (goto _label))))

(event EventBeginPlay
  (CallFunction|SetRandomSpectator)
  (Utilities|Time|SetTimerbyFunctionName 0 "Check If Spectator is Valid" 0.1 true 0.5)
  (Networking|SwitchHasAuthority))

(event Input|AxisEvents|InputAxisLookUp
  (params (AxisValue :type Float%20%28single-precision%29))
  (Pawn|Input|AddControllerPitchInput AxisValue))

(event Input|AxisEvents|InputAxisTurn
  (params (AxisValue :type Float%20%28single-precision%29))
  (Pawn|Input|AddControllerYawInput AxisValue))

(event Input|MouseEvents|LeftMouseButton
  (params (Key :type Key%20Structure :default "None"))
  (bind _returnvalue (Actor|GetAttachParentActor))
  (bind _returnvalue_2 (Game|GetGameState))
  (bind _playerarray (Variables|/Script/Engine.GameStateBase|GetPlayerArray _returnvalue_2))
  (bind _returnvalue_3 (Utilities|Array|Length _playerarray))
  (:Pressed
    (Utilities|IsValid _returnvalue
      (:Is%20Valid
        (bind _asbp_my_golf_ball_player (Utilities|Casting|CastToBP_MyGolfBallPlayer _returnvalue))
        (bind _playerstate (Variables|/Script/Engine.Pawn|GetPlayerState _asbp_my_golf_ball_player)
          (:then
            (for (_array_element _array_index) (Variables|/Script/Engine.GameStateBase|GetPlayerArray (Game|GetGameState))
              (if (== _array_element _playerstate)
                (bind _output_get (Variables|Default|SetSpectating%20Player _array_index))
                (Utilities|FlowControl|ForLoopwithBreak 0 _returnvalue_3 :!label _label
                  (:LoopBody
                    (if (< (Variables|Default|GetSpectating%20Player) _returnvalue_3)
                      (Math|Integer|IncrementInt (Variables|Default|GetSpectating%20Player)
                        (:%20%20
                          (Utilities|IsValid (Utilities|Array|Get(acopy) (Variables|/Script/Engine.GameStateBase|GetPlayerArray (Game|GetGameState)) (Variables|Default|GetSpectating%20Player))
                            (:Is%20Valid
                              (if (not (Variables|/Script/Engine.PlayerState|GetbIsSpectator (Utilities|Array|Get(acopy) (Variables|/Script/Engine.GameStateBase|GetPlayerArray (Game|GetGameState)) (Variables|Default|GetSpectating%20Player))))
                                (Utilities|FlowControl|Sequence ; if it's not a spectator we'll set new spectator parent to him
                                  (:then_0
                                    (goto _label Break))
                                  (:then_1
                                    (Transformation|AttachActorToActor (Variables|/Script/Engine.PlayerState|GetPawnPrivate (Utilities|Array|Get(acopy) (Variables|/Script/Engine.GameStateBase|GetPlayerArray (Game|GetGameState)) (Variables|Default|GetSpectating%20Player))) "None" "SnapToTarget" "SnapToTarget" "SnapToTarget" true))))))))
                      (else
                        (Variables|Default|SetSpectating%20Player -1) ; resets to first index if it surpasses the length of player array
                      )))))))
          (:else))))))

(event Input|MouseEvents|RightMouseButton
  (params (Key :type Key%20Structure :default "None"))
  (bind _returnvalue (Actor|GetAttachParentActor))
  (bind _returnvalue_2 (Game|GetGameState))
  (bind _playerarray (Variables|/Script/Engine.GameStateBase|GetPlayerArray _returnvalue_2))
  (bind _returnvalue_3 (Utilities|Array|Length _playerarray))
  (:Pressed
    (Utilities|IsValid _returnvalue
      (:Is%20Valid
        (bind _asbp_my_golf_ball_player (Utilities|Casting|CastToBP_MyGolfBallPlayer _returnvalue))
        (bind _playerstate (Variables|/Script/Engine.Pawn|GetPlayerState _asbp_my_golf_ball_player)
          (:then
            (for (_array_element _array_index) (Variables|/Script/Engine.GameStateBase|GetPlayerArray (Game|GetGameState))
              (if (== _array_element _playerstate)
                (bind _output_get (Variables|Default|SetSpectating%20Player _array_index))
                (Utilities|FlowControl|ForLoopwithBreak 0 _returnvalue_3 :!label _label
                  (:LoopBody
                    (if (> (Variables|Default|GetSpectating%20Player) -1)
                      (Math|Integer|DecrementInt (Variables|Default|GetSpectating%20Player)
                        (:%20%20
                          (Utilities|IsValid (Utilities|Array|Get(acopy) (Variables|/Script/Engine.GameStateBase|GetPlayerArray (Game|GetGameState)) (Variables|Default|GetSpectating%20Player))
                            (:Is%20Valid
                              (if (not (Variables|/Script/Engine.PlayerState|GetbIsSpectator (Utilities|Array|Get(acopy) (Variables|/Script/Engine.GameStateBase|GetPlayerArray (Game|GetGameState)) (Variables|Default|GetSpectating%20Player))))
                                (Utilities|FlowControl|Sequence ; if it's not a spectator we'll set new spectator parent to him
                                  (:then_0
                                    (goto _label Break))
                                  (:then_1
                                    (Transformation|AttachActorToActor (Variables|/Script/Engine.PlayerState|GetPawnPrivate (Utilities|Array|Get(acopy) (Variables|/Script/Engine.GameStateBase|GetPlayerArray (Game|GetGameState)) (Variables|Default|GetSpectating%20Player))) "None" "SnapToTarget" "SnapToTarget" "SnapToTarget" true))))))))
                      (else
                        (Variables|Default|SetSpectating%20Player _returnvalue_3) ; resets to first index if it surpasses the length of player array
                      )))))))
          (:else))))))

(fn ConstructionScript)