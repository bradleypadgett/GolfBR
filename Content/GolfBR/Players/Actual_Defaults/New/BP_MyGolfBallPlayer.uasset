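; Player golf ball pawn for a multiplayer golf battle-royale game, handling spectator hand-off, name tag and reset.
; It asks BP_GolfBallController to check spectator status and show game-state UI, using a delay hack on possession.
; R stops the ball and teleports it to a fixed point, remote clients show PlayerState names, and events toggle ball-to-ball collision or set arrow rotation.
; Material, arrow colour and end-server events are empty stubs, with old logic left disconnected.
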(event Custom|New%20Golf%20Ball%20Material)

(event Custom|Arrow%20Color)

(event Custom|Kill
  (Physics|SetPhysicsLinearVelocity (Variables|Default|GetGolfBall) "0, 0, 0" false "None")
  (Transformation|SetActorLocation "0, 0,50.000000" false true))

(event Custom|Kill%20self%20as%20client
  (Physics|SetPhysicsLinearVelocity (Variables|Default|GetGolfBall) "0, 0, 0" false "None")
  (Transformation|SetActorLocation "0, 0,50.000000" false true))

(event Custom|Set%20Arrow%20Rotation%20as%20Client
  (params (NewRotation :type Rotator))
  (if (not (Pawn|IsLocallyControlled))
    (Transformation|SetWorldRotation (Variables|Default|GetArrowCenter) NewRotation false false)))

(event Custom|Set%20Client%20Rotation%20as%20Server
  (params (NewRotation :type Rotator))
  (Transformation|SetWorldRotation (Variables|Default|GetArrowCenter) NewRotation false false))

(event Custom|Server%20Start%20Spectating
  (bind _asbp_golf_ball_controller (Utilities|Casting|CastToBP_GolfBallController (Pawn|GetController)))
  (Default|TriggerStartSpectating _asbp_golf_ball_controller))

(event Custom|Update%20Collision
  (params (bIgnore :type Boolean))
  (Collision|SetCollisionResponsetoChannel (Variables|Default|GetGolfBall) "ECC_PhysicsBody" (select bIgnore "ECR_Ignore" "ECR_Block")))

(event Custom|End%20server)

(event EventBeginPlay
  (bind _asbp_golf_ball_controller (Utilities|Casting|CastToBP_GolfBallController (Game|GetPlayerController 0)))
  (Default|CheckifPermanantSpectator _asbp_golf_ball_controller)
  (if true
    (Utilities|Time|SetTimerbyFunctionName 0 "aa" 0.5 true))
  (CallFunction|NewGolfBallMaterial)
  (Utilities|Time|SetTimerbyFunctionName 0 "Arrow Color" 0.05 true)
  (Transformation|SetAbsolute (Variables|Default|GetCameraBoom) false true false))

(event EventTick
  (params (DeltaSeconds :type Float%20%28single-precision%29))
  (Networking|SwitchHasAuthority
    (:Remote
      (bind _asbp_golf_brplayer_state (Utilities|Casting|CastToBP_GolfBRPlayerState (Variables|Default|GetPlayerState)))
      (Rendering|Components|TextRender|SetText (Variables|Default|GetTextRender) (Utilities|Text|ToText(String) (PlayerState|GetPlayerName _asbp_golf_brplayer_state))))))

(event EventPossessed
  (params (NewController :type Controller%20Object%20Reference))
  ;[1 0.1146 0.1146] TOTALLY HACK AND SLASH BUT IT WORKS FOR NOW
  (Utilities|FlowControl|Delay 0.5)
  (bind _asbp_golf_ball_controller (Utilities|Casting|CastToBP_GolfBallController NewController))
  (Default|CheckifPermanantSpectator _asbp_golf_ball_controller)
  (Default|DisplayGameStateUI _asbp_golf_ball_controller))

(event Input|KeyboardEvents|R
  (params (Key :type Key%20Structure))
  (:Pressed
    (Networking|SwitchHasAuthority
      (:Authority
        (CallFunction|Kill))
      (:Remote
        (CallFunction|KillSelfasClient)))))

(event Input|KeyboardEvents|F
  (params (Key :type Key%20Structure))
  (:Pressed
    (CallFunction|EndServer)))

(fn ConstructionScript
  (Variables|Default|SetTesting true))

(fn UpdateArrowRotation)