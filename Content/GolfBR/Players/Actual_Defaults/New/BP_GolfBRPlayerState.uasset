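; Player state for the GolfBR battle royale golf game, tracking round qualification, permanent spectator and lobby status.
; CopyProperties carries QualifiedRound and PermanantSpectator into the new player state, and SetPlayerName builds names from the PlayerArray count.
; Events named for game mode use forward spectator checks and level-choice UI to player controller 0's BP_GolfBallController.
; OnRep_InLobby shows or removes that controller's lobby UI, only on the authority branch.
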(event Custom|Set%20Spectator%20from%20GM
  (bind _asbp_golf_ball_controller (Utilities|Casting|CastToBP_GolfBallController (Game|GetPlayerController 0)))
  (Default|CheckifPermanantSpectator _asbp_golf_ball_controller))

(event Custom|Add%20Choose%20Level%20UI%20from%20GM
  (bind _asbp_golf_ball_controller (Utilities|Casting|CastToBP_GolfBallController (Game|GetPlayerController 0)))
  (Default|DisplayChooseLevelUI _asbp_golf_ball_controller))

(event Custom|Set%20Player%20Name
  (Class|GolfBRPlayerState|SetPlayerNameExposed (Utilities|String|Append "Player " (Utilities|String|ToString(Integer) (Utilities|Array|Length (Variables|/Script/Engine.GameStateBase|GetPlayerArray (Game|GetGameState)))))))

(event EventCopyProperties
  (params (NewPlayerState :type Player%20State%20Object%20Reference))
  (|CallParentFunction NewPlayerState)
  (bind _asbp_golf_brplayer_state (Utilities|Casting|CastToBP_GolfBRPlayerState NewPlayerState))
  (Variables|BP_GolfBRPlayerState_C|SetQualifiedRound _asbp_golf_brplayer_state (Variables|Default|GetQualifiedRound))
  (Variables|BP_GolfBRPlayerState_C|SetPermanantSpectator _asbp_golf_brplayer_state (Variables|Default|GetPermanantSpectator)))

(event EventBeginPlay)

(fn ConstructionScript)

(fn OnRepinLobby
  (bind _asbp_golf_ball_controller (Utilities|Casting|CastToBP_GolfBallController (Game|GetPlayerController 0)))
  (Networking|SwitchHasAuthority
    (:Authority
      (if (Variables|Default|GetInLobby)
        (Default|DisplayLobbyUI _asbp_golf_ball_controller)
        (else
          (Default|RemoveLobbyUI _asbp_golf_ball_controller))))))