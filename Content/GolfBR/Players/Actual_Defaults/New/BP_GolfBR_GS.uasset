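; Game State Blueprint for the GolfBR mode, apparently meant to track round completion and player qualification.
; Events flag the round as ready to end, set a qualification value and increment a qualified-player count with a debug print.
; The logic is largely unfinished: the players-left loop over PlayerArray has an empty body with a disconnected PlayerState cast, and the round-parameter and unqualified-player events are empty stubs.
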(event Custom|Initialize%20Round%20Params)

(event Custom|Set%20Unqualified%20Players)

(event Custom|Initialize%20Amount%20to%20Qualify
  (params (NewParam :type Integer))
  (Variables|Default|Set/# NewParam))

(event Custom|Get%20Players%20Left
  (for _array_element (Variables|Default|GetPlayerArray)
    _))

(event Custom|Ready%20to%20End%20Round
  (Variables|Default|SetbReady%20to%20End%20Round true))

(event Custom|Add%20Qualified%20Player%20Amount
  (Math|Integer|IncrementInt (Variables|Default|Get#/)
    (:%20%20
      (Development|PrintString "BBBBBBBBBBBRUH22222"))))

(event EventBeginPlay)

(event EventTick
  (params (DeltaSeconds :type Float%20%28single-precision%29)))

(fn ConstructionScript)