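; Game mode for the putt-putt round of GolfBR, a golf battle royale, which sets how many players qualify.
; At match start it labels the game state "Qualified", counts players who are not permanent spectators, and sets the qualify limit to one fewer.
; ReadyToEndMatch compares a game state value against that limit, and EndPlay calls the game state's ReadyToEndRound.
; The logout round check is a stub, and debug prints and disconnected logic remain.
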(event Custom|Check%20Round%20End
  (Utilities|Casting|CastToBP_GolfBR_PuttPutt (Game|GetGameState)))

(event EventBeginPlay
  (|CallParentFunction))

(event EventTick
  (params (DeltaSeconds :type Float%20%28single-precision%29))
  (|CallParentFunction DeltaSeconds) ; This node is disabled and will not be called.\nDrag off pins to build functionality.
)

(event EventRoundEnded
  (|CallParentFunction))

(event EventOnLogout
  (params (ExitingController :type Controller%20Object%20Reference))
  (CallFunction|CheckRoundEnd))

(event EventEndPlay
  (params (EndPlayReason :type EEndPlayReason%20Enum :default "Destroyed"))
  (bind _asbp_golf_br_putt_putt (Utilities|Casting|CastToBP_GolfBR_PuttPutt (Game|GetGameState)))
  (Default|ReadytoEndRound _asbp_golf_br_putt_putt)
  (|CallParentFunction EndPlayReason))

(event EventOnSetMatchState
  (params (NewState :type Name :default "None"))
  (if (Class|GameModeBase|HasMatchEnded)
    (CallFunction|RoundEnded)
    (elif (Class|GameModeBase|HasMatchStarted)
      _)))

(event EventPostLogin
  (params (NewPlayer :type Player%20Controller%20Object%20Reference))
  (|CallParentFunction NewPlayer))

(event EventBPPostSeamlessTravel)

(event EventBPHandleMatchHasStarted
  (bind _returnvalue (Game|GetGameState))
  (bind _qualify_max_temp (Variables|Default|Getqualify%20max%20temp))
  (|CallParentFunction)
  (bind _asgs_golf_br (Utilities|Casting|CastToGS_GolfBR _returnvalue))
  (Variables|Default|SetAs%20GS%20Golf%20BR _asgs_golf_br)
  (bind _asbp_golf_br_putt_putt (Utilities|Casting|CastToBP_GolfBR_PuttPutt _returnvalue)
    (:then
      (Variables|/Game/GolfBR/Players/Actual_Defaults/New/BP_GolfBR_GS.BP_GolfBR_GS_C|SetQualify%20Text _asbp_golf_br_putt_putt "Qualified"))
    (:CastFailed
      _))
  (Development|PrintString (Utilities|String|Append "AAAAAAAAAAAAAA" " " (Utilities|String|ToString(Integer) (Utilities|Array|Length (Class|GSGolfBR|GetPlayers (Variables|Default|GetAs%20GS%20Golf%20BR)))) "////" (Utilities|String|ToString(Integer) (Variables|Default|GetNumTravellingPlayers)) "//////" (Utilities|String|ToString(Integer) (Variables|Default|GetNumPlayers))))
  (for _array_element (Class|GSGolfBR|GetPlayers (Variables|Default|GetAs%20GS%20Golf%20BR))
    (bind _asbp_golf_brplayer_state (Utilities|Casting|CastToBP_GolfBRPlayerState _array_element))
    (if (not (Variables|/Game/GolfBR/Players/Actual_Defaults/New/BP_GolfBRPlayerState.BP_GolfBRPlayerState_C|GetPermanantSpectator _asbp_golf_brplayer_state))
      (Math|Integer|IncrementInt (Variables|Default|Getqualify%20max%20temp))))
  (Math|Integer|DecrementInt _qualify_max_temp
    (:%20%20
      (Variables|Default|SetMax%20Qualify _qualify_max_temp)
      (bind _asbp_golf_br_putt_putt_2 (Utilities|Casting|CastToBP_GolfBR_PuttPutt (Game|GetGameState)))
      (Variables|/Game/GolfBR/Players/Actual_Defaults/New/BP_GolfBR_GS.BP_GolfBR_GS_C|Set/# _asbp_golf_br_putt_putt_2 (Variables|Default|Getqualify%20max%20temp)))))

(fn ConstructionScript
  (|CallParentFunction))

(fn ReadytoEndMatch
  (bind _asbp_golf_br_putt_putt (Utilities|Casting|CastToBP_GolfBR_PuttPutt (Game|GetGameState)))
  (return (>= (Variables|/Game/GolfBR/Players/Actual_Defaults/New/BP_GolfBR_GS.BP_GolfBR_GS_C|Get#/ _asbp_golf_br_putt_putt) (Variables|Default|GetMax%20Qualify))))

(fn ReadytoStartMatch
  (bind _returnvalue (|CallParentFunction))
  (return _returnvalue))