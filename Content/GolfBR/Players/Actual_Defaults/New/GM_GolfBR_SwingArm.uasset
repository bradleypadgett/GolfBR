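; Game mode for the SwingArm round of the golf battle royale, an elimination-labelled mode.
; On match start it sets the game state's text to "Eliminated", counts non-spectator players, and derives MaxQualify as that count minus two, also copying it to the game state.
; ReadyToEndMatch compares a game-state value against MaxQualify.
; A match-end state triggers the parent's RoundEnded, and EndPlay calls the game state's ReadyToEndRound.
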(event Custom|Check%20Round%20End)

(event EventBeginPlay
  (|CallParentFunction))

(event EventTick
  (params (DeltaSeconds :type Float%20%28single-precision%29))
  (|CallParentFunction DeltaSeconds) ; This node is disabled and will not be called.\nDrag off pins to build functionality.
)

(event EventRoundEnded
  (|CallParentFunction))

(event EventOnLogout
  (params (ExitingController :type Controller%20Object%20Reference))
  (CallFunction|CheckRoundEnd))

(event EventEndPlay
  (params (EndPlayReason :type EEndPlayReason%20Enum :default "Destroyed"))
  (bind _asbp_golf_br_gs_swing_arm (Utilities|Casting|CastToBP_GolfBR_GS_SwingArm (Game|GetGameState)))
  (Default|ReadytoEndRound _asbp_golf_br_gs_swing_arm)
  (|CallParentFunction EndPlayReason))

(event EventOnSetMatchState
  (params (NewState :type Name :default "None"))
  (if (Class|GameModeBase|HasMatchEnded)
    (CallFunction|RoundEnded)
    (elif (Class|GameModeBase|HasMatchStarted)
      _)))

(event EventPostLogin
  (params (NewPlayer :type Player%20Controller%20Object%20Reference))
  (|CallParentFunction NewPlayer))

(event EventBPPostSeamlessTravel)

(event EventBPHandleMatchHasStarted
  (bind _returnvalue (Game|GetGameState))
  (bind _playerarray (Variables|/Script/Engine.GameStateBase|GetPlayerArray _returnvalue))
  (|CallParentFunction)
  (bind _asbp_golf_br_gs_swing_arm (Utilities|Casting|CastToBP_GolfBR_GS_SwingArm _returnvalue)
    (:then
      (Variables|/Game/GolfBR/Players/Actual_Defaults/New/BP_GolfBR_GS.BP_GolfBR_GS_C|SetQualify%20Text _asbp_golf_br_gs_swing_arm "Eliminated"))
    (:CastFailed
      _))
  (Development|PrintString (Utilities|String|Append "AAAAAAAAAAAAAA" " " (Utilities|String|ToString(Integer) (Utilities|Array|Length _playerarray)) "////" (Utilities|String|ToString(Integer) (Variables|Default|GetNumTravellingPlayers)) "//////" (Utilities|String|ToString(Integer) (Variables|Default|GetNumPlayers))))
  (for _array_element _playerarray
    (bind _asbp_golf_brplayer_state (Utilities|Casting|CastToBP_GolfBRPlayerState _array_element))
    (if (not (Variables|/Game/GolfBR/Players/Actual_Defaults/New/BP_GolfBRPlayerState.BP_GolfBRPlayerState_C|GetPermanantSpectator _asbp_golf_brplayer_state))
      (Math|Integer|IncrementInt (Variables|Default|Getqualify%20max%20temp))))
  (Variables|Default|Setqualify%20max%20temp (- (Variables|Default|Getqualify%20max%20temp) 2))
  (Variables|Default|SetMax%20Qualify (Variables|Default|Getqualify%20max%20temp))
  (bind _asbp_golf_br_gs_swing_arm_2 (Utilities|Casting|CastToBP_GolfBR_GS_SwingArm _returnvalue))
  (Variables|/Game/GolfBR/Players/Actual_Defaults/New/BP_GolfBR_GS.BP_GolfBR_GS_C|Set/# _asbp_golf_br_gs_swing_arm_2 (Variables|Default|Getqualify%20max%20temp)))

(fn ConstructionScript
  (|CallParentFunction))

(fn ReadytoEndMatch
  (bind _asbp_golf_br_gs_swing_arm (Utilities|Casting|CastToBP_GolfBR_GS_SwingArm (Game|GetGameState)))
  (return (>= (Variables|/Game/GolfBR/Players/Actual_Defaults/New/BP_GolfBR_GS.BP_GolfBR_GS_C|Get#/ _asbp_golf_br_gs_swing_arm) (Variables|Default|GetMax%20Qualify))))

(fn ReadytoStartMatch
  (bind _returnvalue (|CallParentFunction))
  (return _returnvalue))