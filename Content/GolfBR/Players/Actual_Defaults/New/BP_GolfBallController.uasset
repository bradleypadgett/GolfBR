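; Player controller for the golf battle royale that handles round qualification, spectating and per-player UI.
; Qualifying sets the PlayerState flag, increments the GameState's qualified count and starts spectating; a permanent-spectator check also toggles spectating.
; Spectator switches cache the golf ball pawn, update its collision and swap gameplay and spectator widgets.
; Possession triggers a delayed lobby check that shows game-state UI outside the lobby.
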(event Custom|Set%20Qualified%20test
  (bind _asbp_golf_brplayer_state (Utilities|Casting|CastToBP_GolfBRPlayerState (Variables|Default|GetPlayerState)))
  (Variables|/Game/GolfBR/Players/Actual_Defaults/New/BP_GolfBRPlayerState.BP_GolfBRPlayerState_C|SetQualifiedRound _asbp_golf_brplayer_state true))

(event Custom|Qualify%20Player
  (bind _asbp_golf_brplayer_state (Utilities|Casting|CastToBP_GolfBRPlayerState (Variables|Default|GetPlayerState)))
  (bind _output_get (Variables|/Game/GolfBR/Players/Actual_Defaults/New/BP_GolfBRPlayerState.BP_GolfBRPlayerState_C|SetQualifiedRound _asbp_golf_brplayer_state true))
  (Development|PrintString (Utilities|String|Append "BBBBRUH I AM" (Utilities|String|ToString(Boolean) _output_get)))
  (bind _asbp_golf_br_gs (Utilities|Casting|CastToBP_GolfBR_GS (Game|GetGameState))
    (:then
      (Default|AddQualifiedPlayerAmount _asbp_golf_br_gs)
      (Development|PrintString "BBBBBBBBBBBRUH"))
    (:CastFailed
      _))
  (CallFunction|TriggerStartSpectating))

(event EventTick
  (params (DeltaSeconds :type Float%20%28single-precision%29)))

(event EventBeginPlay)

(event EventPossess
  (params (PossessedPawn :type Pawn%20Object%20Reference))
  (|CallParentFunction PossessedPawn)
  (Utilities|FlowControl|Delay 0.5)
  (CallFunction|CheckifinLobby))

(event Input|KeyboardEvents|E
  (params (Key :type Key%20Structure :default "None")))

(event Custom|Trigger%20Stop%20Spectating
  (Class|GolfBallController|ChangeStatetoPlayer)
  (CallFunction|DisplayGameUI)
  (bind _asbp_my_golf_ball_player (Utilities|Casting|CastToBP_MyGolfBallPlayer (Variables|Default|GetOldPawn)))
  (Default|UpdateCollision _asbp_my_golf_ball_player false))

(event Custom|Display%20Game%20UI
  (bind _returnvalue (UserInterface|CreateWidget "/Game/GolfBR/UI/UI_TestGameplay.UI_TestGameplay_C"))
  (bind _output_get (Variables|Default|SetGame%20UI _returnvalue))
  (UserInterface|Viewport|AddtoViewport _output_get 0)
  (bind _spectator_ui (Variables|Default|GetSpectator%20UI)
    (:then
      (Widget|RemovefromParent _spectator_ui))
    (:else
      _))
  (bind _lobby_ui (Variables|Default|GetLobby%20UI)
    (:then
      (Widget|RemovefromParent _lobby_ui))
    (:else)))

(event Custom|Display%20Spectating%20UI
  (bind _returnvalue (UserInterface|CreateWidget "/Game/GolfBR/UI/UI_Spectator.UI_Spectator_C"))
  (bind _output_get (Variables|Default|SetSpectator%20UI _returnvalue))
  (UserInterface|Viewport|AddtoViewport _output_get 0)
  (bind _foundwidgets (Widget|GetAllWidgetsOfClass "/Game/GolfBR/UI/UI_TestGameplay.UI_TestGameplay_C" true))
  (for _array_element _foundwidgets
    (Widget|RemovefromParent _array_element))
  (bind _game_ui (Variables|Default|GetGame%20UI)
    (:then
      (Widget|RemovefromParent _game_ui))
    (:else
      _))
  (bind _lobby_ui (Variables|Default|GetLobby%20UI)
    (:then
      (Widget|RemovefromParent _lobby_ui))
    (:else)))

(event Custom|Check%20if%20Permanant%20Spectator
  (bind _asbp_golf_brplayer_state (Utilities|Casting|CastToBP_GolfBRPlayerState (Variables|Default|GetPlayerState)))
  (Development|PrintString (Utilities|String|Append "Am I a spectator? " (Utilities|String|ToString(Boolean) (Variables|/Game/GolfBR/Players/Actual_Defaults/New/BP_GolfBRPlayerState.BP_GolfBRPlayerState_C|GetPermanantSpectator _asbp_golf_brplayer_state))))
  (if (Variables|/Game/GolfBR/Players/Actual_Defaults/New/BP_GolfBRPlayerState.BP_GolfBRPlayerState_C|GetPermanantSpectator _asbp_golf_brplayer_state)
    (CallFunction|TriggerStartSpectating)
    (else
      (CallFunction|TriggerStopSpectating))))

(event Custom|Check%20if%20In%20Lobby
  (bind _asbp_golf_brplayer_state (Utilities|Casting|CastToBP_GolfBRPlayerState (Variables|Default|GetPlayerState)))
  (if (not (Variables|/Game/GolfBR/Players/Actual_Defaults/New/BP_GolfBRPlayerState.BP_GolfBRPlayerState_C|GetInLobby _asbp_golf_brplayer_state))
    (CallFunction|DisplayGameStateUI)))

(event Custom|Display%20Lobby%20UI
  (bind _returnvalue (UserInterface|CreateWidget "/Game/GolfBR/Players/Actual_Defaults/New/GameStarting/WBP_Lobby.WBP_Lobby_C"))
  (bind _output_get (Variables|Default|SetLobby%20UI _returnvalue))
  (UserInterface|Viewport|AddtoViewport _output_get 0))

(event Custom|Remove%20Lobby%20UI
  (bind _foundwidgets (Widget|GetAllWidgetsOfClass "/Game/GolfBR/Players/Actual_Defaults/New/GameStarting/WBP_Lobby.WBP_Lobby_C" true))
  (for _array_element _foundwidgets
    (Widget|RemovefromParent _array_element)))

(event Custom|Trigger%20Start%20Spectating
  (bind _output_get (Variables|Default|SetOldPawn (Pawn|GetControlledPawn))) ; Server's pawn
  (bind _asbp_my_golf_ball_player (Utilities|Casting|CastToBP_MyGolfBallPlayer _output_get))
  (Default|UpdateCollision _asbp_my_golf_ball_player true)
  (Class|GolfBallController|ChangeStatetoSpectator) ; This will change player to spectator | Spectator will then initialize
  (CallFunction|DisplaySpectatingUI))

(event Custom|Display%20GameState%20UI
  (bind _returnvalue (UserInterface|CreateWidget "/Game/GolfBR/Players/Actual_Defaults/New/GameStateUI.GameStateUI_C"))
  (bind _output_get (Variables|Default|SetGameState%20UI _returnvalue))
  (UserInterface|Viewport|AddtoViewport _output_get 0))

(event Custom|Display%20Choose%20Level%20UI
  (bind _returnvalue (UserInterface|CreateWidget "/Game/GolfBR/Players/Actual_Defaults/New/Transition/ChooseLevelUI.ChooseLevelUI_C"))
  (bind _output_get (Variables|Default|SetChooselevel%20UI _returnvalue))
  (UserInterface|Viewport|AddtoViewport _output_get 0))

(fn ConstructionScript)