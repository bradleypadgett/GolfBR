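; Putt-putt round class for the GolfBR mode, which eliminates players who fail to qualify when the round ends.
; On BeginPlay the authority sets the qualify text.
; At round end it flags each unqualified BP_GolfBRPlayerState as a permanent spectator, leaves existing spectators as they are, then calls the parent logic.
; Round parameter setup computes a rounded share of the player count but never stores it.
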(event EventBeginPlay
  (|CallParentFunction)
  (Networking|SwitchHasAuthority
    (:Authority
      (Variables|Default|SetQualify%20Text "Qualifieed"))))

(event EventTick
  (params (DeltaSeconds :type Float%20%28single-precision%29))
  (|CallParentFunction DeltaSeconds) ; This node is disabled and will not be called.\nDrag off pins to build functionality.
)

(event EventReadytoEndRound
  (for _array_element (Variables|Default|GetPlayerArray)
    (Utilities|IsValid _array_element
      (:Is%20Valid
        (bind _asbp_golf_brplayer_state (Utilities|Casting|CastToBP_GolfBRPlayerState _array_element))
        (if (not (Variables|/Game/GolfBR/Players/Actual_Defaults/New/BP_GolfBRPlayerState.BP_GolfBRPlayerState_C|GetPermanantSpectator _asbp_golf_brplayer_state))
          (Variables|/Game/GolfBR/Players/Actual_Defaults/New/BP_GolfBRPlayerState.BP_GolfBRPlayerState_C|SetPermanantSpectator _asbp_golf_brplayer_state (select (Variables|/Game/GolfBR/Players/Actual_Defaults/New/BP_GolfBRPlayerState.BP_GolfBRPlayerState_C|GetQualifiedRound _asbp_golf_brplayer_state) false true))))))
  (|CallParentFunction))

(event EventInitializeRoundParams
  (Variables|Default|Set/# (Math|Float|Round (* (Math|Conversions|ToFloat(Integer) (Utilities|Array|Length (Variables|Default|GetPlayerArray))) 0.8))))

(fn ConstructionScript
  (|CallParentFunction))