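; BP_GolfBR_GS_FallingPlatform is the Falling Platform game state for the GolfBR mode, handling end-of-round spectator status.
; On ReadytoEndRound it loops through the GS_GolfBR player list and sets PermanantSpectator to match QualifiedRound for players not already permanent spectators, so qualified players become spectators.
; It then calls the parent round-end logic; a Delay before that call is left unconnected.
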(event EventBeginPlay
  (|CallParentFunction) ; This node is disabled and will not be called.\nDrag off pins to build functionality.
)

(event EventTick
  (params (DeltaSeconds :type Float%20%28single-precision%29))
  (|CallParentFunction DeltaSeconds) ; This node is disabled and will not be called.\nDrag off pins to build functionality.
)

(event EventReadytoEndRound
  (bind _asgs_golf_br (Utilities|Casting|CastToGS_GolfBR (Game|GetGameState)))
  (for _array_element (Class|GSGolfBR|GetPlayers _asgs_golf_br)
    (Utilities|IsValid _array_element
      (:Is%20Valid
        (bind _asbp_golf_brplayer_state (Utilities|Casting|CastToBP_GolfBRPlayerState _array_element))
        (if (not (Variables|/Game/GolfBR/Players/Actual_Defaults/New/BP_GolfBRPlayerState.BP_GolfBRPlayerState_C|GetPermanantSpectator _asbp_golf_brplayer_state))
          (Variables|/Game/GolfBR/Players/Actual_Defaults/New/BP_GolfBRPlayerState.BP_GolfBRPlayerState_C|SetPermanantSpectator _asbp_golf_brplayer_state (select (Variables|/Game/GolfBR/Players/Actual_Defaults/New/BP_GolfBRPlayerState.BP_GolfBRPlayerState_C|GetQualifiedRound _asbp_golf_brplayer_state) true false))))))
  (|CallParentFunction))

(fn ConstructionScript
  (|CallParentFunction))