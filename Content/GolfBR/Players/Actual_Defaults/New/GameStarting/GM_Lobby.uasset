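; GM_Lobby is the lobby game mode that gathers players and server-travels them to L_PuttPutt_1.
; On login it sets each player state's name and InLobby flag, clearing the flag when player controllers are swapped.
; The match becomes ready at PlayersToStart, then Tick starts a one-shot countdown timeline that travels on finish.
; Reaching MaxPlayers after the match starts stops the countdown and travels immediately.
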(event EventBeginPlay
  (Utilities|Casting|CastToGS_Lobby (Game|GetGameState)))

(event EventTick
  (params (DeltaSeconds :type Float%20%28single-precision%29))
  (if (Class|GameModeBase|HasMatchStarted)
    (Utilities|FlowControl|Sequence
      (:then_0
        (Utilities|FlowControl|DoOnce false
          (:Completed
            (Timeline|Start%20Match%20Countdown Play
              (:Finished
                (Development|ExecuteConsoleCommand "ServerTravel L_PuttPutt_1" 0 :!label _label))))))
      (:then_1
        (if (>= (Utilities|Array|Length (Variables|/Script/Engine.GameStateBase|GetPlayerArray (Game|GetGameState))) (Variables|Default|GetMax%20Players))
          (Utilities|FlowControl|DoOnce false
            (:Completed
              (Utilities|FlowControl|Sequence
                (:then_0
                  (Timeline|Start%20Match%20Countdown Stop))
                (:then_1
                  (goto _label))))))))))

(event EventPostLogin
  (params (NewPlayer :type Player%20Controller%20Object%20Reference))
  (bind _playerstate (Variables|/Script/Engine.Controller|GetPlayerState NewPlayer)
    (:then
      (bind _asbp_golf_brplayer_state (Utilities|Casting|CastToBP_GolfBRPlayerState _playerstate))
      (Default|SetPlayerName _asbp_golf_brplayer_state)
      (Variables|/Game/GolfBR/Players/Actual_Defaults/New/BP_GolfBRPlayerState.BP_GolfBRPlayerState_C|SetInLobby _asbp_golf_brplayer_state true))
    (:else)))

(event EventOnSwapPlayerControllers
  (params (OldPC :type Player%20Controller%20Object%20Reference) (NewPC :type Player%20Controller%20Object%20Reference))
  (bind _asbp_golf_brplayer_state (Utilities|Casting|CastToBP_GolfBRPlayerState (Variables|/Script/Engine.Controller|GetPlayerState OldPC)))
  (Variables|/Game/GolfBR/Players/Actual_Defaults/New/BP_GolfBRPlayerState.BP_GolfBRPlayerState_C|SetInLobby _asbp_golf_brplayer_state false)
  (|CallParentFunction OldPC NewPC))

(fn ConstructionScript)

(fn ReadytoStartMatch
  (return (>= (Utilities|Array|Length (Variables|/Script/Engine.GameStateBase|GetPlayerArray (Game|GetGameState))) (Variables|Default|GetPlayers%20to%20Start))))

(fn OnRepMaxPlayers)