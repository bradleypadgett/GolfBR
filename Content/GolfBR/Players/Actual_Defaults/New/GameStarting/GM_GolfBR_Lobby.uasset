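; Lobby game mode for GolfBR that gathers players, then server-travels them to the level-choice map.
; It copies MaxPlayers to GS_Lobby, and on login sets each player's name and shows the lobby UI.
; The match starts at PlayersToStart, running a Timeline as a countdown that a full lobby cuts short.
; Players' InLobby flags are cleared before travel and on controller swap.
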(event EventBeginPlay
  (bind _asgs_lobby (Utilities|Casting|CastToGS_Lobby (Game|GetGameState)))
  (Variables|/Game/GolfBR/Players/Actual_Defaults/New/GameStarting/GS_Lobby.GS_Lobby_C|SetMax%20Players _asgs_lobby (Variables|Default|GetMax%20Players)))

(event EventTick
  (params (DeltaSeconds :type Float%20%28single-precision%29))
  (if (Class|GameModeBase|HasMatchStarted)
    (Utilities|FlowControl|Sequence
      (:then_0
        (Utilities|FlowControl|DoOnce false
          (:Completed
            (Timeline|Timeline_0 Play
              (:Finished
                (for _array_element (Variables|/Script/Engine.GameStateBase|GetPlayerArray (Game|GetGameState)) :!label _label
                  (bind _asbp_golf_brplayer_state (Utilities|Casting|CastToBP_GolfBRPlayerState _array_element))
                  (Variables|/Game/GolfBR/Players/Actual_Defaults/New/BP_GolfBRPlayerState.BP_GolfBRPlayerState_C|SetInLobby _asbp_golf_brplayer_state false))
                (Development|ExecuteConsoleCommand "ServerTravel L_ChooseLevelMap" 0))))))
      (:then_1
        (if (>= (Utilities|Array|Length (Variables|/Script/Engine.GameStateBase|GetPlayerArray (Game|GetGameState))) (Variables|Default|GetMax%20Players))
          (Utilities|FlowControl|DoOnce false
            (:Completed
              (Utilities|FlowControl|Sequence
                (:then_0
                  (Timeline|Timeline_0 Stop))
                (:then_1
                  (goto _label))))))))))

(event EventPostLogin
  (params (NewPlayer :type Player%20Controller%20Object%20Reference))
  (bind _playerstate (Variables|/Script/Engine.Controller|GetPlayerState NewPlayer)
    (:then
      (bind _asbp_golf_brplayer_state (Utilities|Casting|CastToBP_GolfBRPlayerState _playerstate))
      (Default|SetPlayerName _asbp_golf_brplayer_state)
      (|CallParentFunction NewPlayer)
      (bind _asbp_golf_ball_controller (Utilities|Casting|CastToBP_GolfBallController NewPlayer))
      (Default|DisplayLobbyUI _asbp_golf_ball_controller))
    (:else)))

(event EventOnSwapPlayerControllers
  (params (OldPC :type Player%20Controller%20Object%20Reference) (NewPC :type Player%20Controller%20Object%20Reference))
  (bind _asbp_golf_brplayer_state (Utilities|Casting|CastToBP_GolfBRPlayerState (Variables|/Script/Engine.Controller|GetPlayerState OldPC)))
  (Variables|/Game/GolfBR/Players/Actual_Defaults/New/BP_GolfBRPlayerState.BP_GolfBRPlayerState_C|SetInLobby _asbp_golf_brplayer_state false)
  (|CallParentFunction OldPC NewPC))

(fn ConstructionScript
  (|CallParentFunction))

(fn ReadytoStartMatch
  (return (>= (Utilities|Array|Length (Variables|/Script/Engine.GameStateBase|GetPlayerArray (Game|GetGameState))) (Variables|Default|GetPlayers%20to%20Start))))