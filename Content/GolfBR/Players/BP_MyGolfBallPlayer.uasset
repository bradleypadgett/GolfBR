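; Player Blueprint for a golf ball, with a camera boom, a direction arrow and a color-cycling look.
; On BeginPlay it gives the ball a dynamic material, adds the main UI widget to the viewport and sets the boom and ball to absolute rotation.
; A fast looping timer runs ArrowColor, which advances a hue to recolor the ball material and arrow and stores a UI color.
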(event Custom|New%20Golf%20Ball%20Material
  (bind _returnvalue (Rendering|Material|CreateDynamicMaterialInstance (Variables|Default|GetGolfBall) 0 "/Game/StarterContent/Materials/M_Basic_Wall.M_Basic_Wall" "None" :!class /Script/Engine.PrimitiveComponent))
  (Variables|Default|Setgolfballmat _returnvalue)
  (Rendering|Material|SetMaterial (Variables|Default|GetGolfBall) 0 (Variables|Default|Getgolfballmat)))

(event Custom|Arrow%20Color
  (bind _output_get (Variables|Default|Sethue (+ (Variables|Default|Gethue) 2.0)))
  (Rendering|Material|SetVectorParameterValue (Variables|Default|Getgolfballmat) "Color" (Class|KismetMathLibrary|HSVtoRGB (+ _output_get 15.0) 1.0 0.8 1.0) :!class /Script/Engine.MaterialInstanceDynamic)
  (Components|Arrow|SetArrowColor(LinearColor) (Variables|Default|GetArrow) (Class|KismetMathLibrary|HSVtoRGB _output_get 1.0 0.8 1.0))
  (Variables|Default|Setui%20clor (Class|KismetMathLibrary|HSVtoRGB _output_get 1.0 0.8 1.0)))

(event EventBeginPlay
  (CallFunction|NewGolfBallMaterial)
  (Utilities|Time|SetTimerbyFunctionName 0 "Arrow Color" 0.05 true)
  (bind _returnvalue (UserInterface|CreateWidget "/Game/GolfBR/UI/PB_MainUI.PB_MainUI_C" (Game|GetPlayerController 0)))
  (UserInterface|Viewport|AddtoViewport _returnvalue 0)
  (Transformation|SetAbsolute (Variables|Default|GetCameraBoom) false true false))

(event EventTick
  (params (DeltaSeconds :type Float%20%28single-precision%29)))

(fn ConstructionScript)