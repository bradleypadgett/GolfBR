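; BP_TestPlayer is a test golf-ball player, launched with F along movement input relative to camera yaw, defaulting to forward.
; R zeroes the ball's velocity and teleports it to a fixed point, branching on authority.
; Tick smoothly rotates the aim arrow using camera yaw and an input-zero check that is reversed from the launch's.
; Arrow colour cycling, ball material, HUD creation and most arrow-sync logic are disconnected.
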(event Custom|New%20Golf%20Ball%20Material)

(event Custom|Arrow%20Color)

(event Custom|Kill
  (Physics|SetPhysicsLinearVelocity (Variables|Default|GetGolfBall) "0, 0, 0" false "None")
  (Transformation|SetActorLocation "0, 0,50.000000" false true))

(event Custom|Kill%20self%20as%20client
  (Physics|SetPhysicsLinearVelocity (Variables|Default|GetGolfBall) "0, 0, 0" false "None")
  (Transformation|SetActorLocation "0, 0,50.000000" false true))

(event Custom|Set%20Arrow%20Rotation%20as%20Client
  (params (NewRotation :type Rotator))
  (if (not (Pawn|IsLocallyControlled))
    (Transformation|SetWorldRotation (Variables|Default|GetArrowCenter) NewRotation false false)))

(event Custom|Set%20Client%20Rotation%20as%20Server
  (params (NewRotation :type Rotator))
  (Transformation|SetWorldRotation (Variables|Default|GetArrowCenter) NewRotation false false))

(event EventBeginPlay
  (CallFunction|NewGolfBallMaterial)
  (Utilities|Time|SetTimerbyFunctionName 0 "Arrow Color" 0.05 true)
  (Transformation|SetAbsolute (Variables|Default|GetCameraBoom) false true false))

(event EventTick
  (params (DeltaSeconds :type Float%20%28single-precision%29))
  (CallFunction|UpdateArrowRotation DeltaSeconds))

(event Input|AxisEvents|InputAxisLookUp
  (params (AxisValue :type Float%20%28single-precision%29))
  (Pawn|Input|AddControllerPitchInput AxisValue))

(event Input|AxisEvents|InputAxisTurn
  (params (AxisValue :type Float%20%28single-precision%29))
  (Pawn|Input|AddControllerYawInput AxisValue))

(event Input|KeyboardEvents|R
  (params (Key :type Key%20Structure))
  (:Pressed
    (Networking|SwitchHasAuthority
      (:Authority
        (CallFunction|Kill))
      (:Remote
        (CallFunction|KillSelfasClient)))))

(event Input|KeyboardEvents|F
  (params (Key :type Key%20Structure))
  (bind _returnvalue (Input|AxisValues|GetMoveForward))
  (bind _returnvalue_2 (Input|AxisValues|GetMoveRight))
  (bind _returnvalue_3 (Math|Vector|MakeVector _returnvalue _returnvalue_2 0.0))
  (:Pressed
    (Physics|AddImpulse (Variables|Default|GetGolfBall) (* (Math|Vector|RotateVectorAroundAxis (select (Math|Vector|Equal(Vector) _returnvalue_3 "0, 0, 0" 0.0001) "1.000000, 0, 0" _returnvalue_3) (.yaw (Transformation|GetWorldRotation (Variables|Default|GetFollowCamera))) "0, 0,1.000000") 1e+03) "None" true)))

(fn ConstructionScript)

(fn UpdateArrowRotation
  (params (DeltaTime :type Float%20%28single-precision%29))
  (bind _returnvalue (Input|AxisValues|GetMoveRight))
  (bind _returnvalue_2 (Input|AxisValues|GetMoveForward))
  (bind _returnvalue_3 (Math|Vector|MakeVector _returnvalue_2 _returnvalue 0.0))
  (Transformation|SetWorldRotation (Variables|Default|GetArrowCenter) (Math|Interpolation|RInterpTo (Transformation|GetWorldRotation (Variables|Default|GetArrowCenter)) (Math|Rotator|MakeRotfromX (Math|Vector|RotateVectorAroundAxis (select (Math|Vector|Equal(Vector) "0, 0, 0" _returnvalue_3 0.0001) _returnvalue_3 "1.000000, 0, 0") (.yaw (Transformation|GetWorldRotation (Variables|Default|GetFollowCamera))) "0, 0,1.000000")) DeltaTime 1e+01) false false))